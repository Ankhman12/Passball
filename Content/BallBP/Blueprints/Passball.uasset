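; Passball is a networked throwable bomb ball that first-person characters carry, throw and intercept, with materials showing its state.
; A hit from a character triggers pickup, attaching the ball to their camera, and ThrowBall restores physics and applies an impulse.
; Server tick uses a sphere overlap to detect "Ground"-tagged meshes and runs a fuse while active.
; Pickup by another character resets the fuse; expiry detaches the ball and launches nearby characters.
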(event Custom|HitEvent_Multi
  (Utilities|IsValid (stale Collision|EventHit Other)
    (:Is%20Valid
      (bind _asfirst_person_character (Utilities|Casting|CastToFirstPersonCharacter (stale Collision|EventHit Other)))
      (CallFunction|BallPickup _asfirst_person_character))))

(event Custom|EventStart_Server
  (Rendering|Material|SetMaterial (Variables|Default|GetBall_Mesh) 0 "/Game/BallBP/Materials/Ball-Stasis.Ball-Stasis")
  (Variables|Default|SetBallState "NewEnumerator3")
  (Physics|SetEnableGravity (Variables|Default|GetBall_Mesh) false)
  (Physics|SetSimulatePhysics (Variables|Default|GetBall_Mesh) false)
  (Class|PrimitiveComponent|SetUseCCD (Variables|Default|GetBall_Mesh) true "None"))

(event Custom|TickEvent_Server
  (Utilities|FlowControl|Sequence
    (:then_0
      (if (Utilities|IsBallActive)
        (bind _output_get (Variables|Default|SetBallTimer (+ (Variables|Default|GetBallTimer) (Variables|Default|GetdeltaTime))))
        (if (>= _output_get (Variables|Default|GetMaxTime))
          (CallFunction|Explode))))
    (:then_1
      (if (not (Math|Boolean|ORBoolean (Utilities|Enum|Equal(Enum) (Variables|Default|GetBallState) "NewEnumerator0") (Utilities|Enum|Equal(Enum) (Variables|Default|GetBallState) "NewEnumerator3") (Variables|Default|GethasExploded)))
        (bind (_outactors _returnvalue) (Collision|SphereOverlapActors (Transformation|GetWorldLocation (Variables|Default|GetBall_Mesh)) 75.0 (Utilities|Array|MakeArray "ObjectTypeQuery1") "/Script/Engine.StaticMeshActor"))
        (if _returnvalue
          (bind _array_element (Utilities|Array|ForEachLoopwithBreak _outactors :!label _label)
            (:LoopBody
              (Utilities|IsValid _array_element
                (:Is%20Valid
                  (if (Components|ComponentHasTag (Actor|GetComponentbyClass _array_element "/Script/Engine.StaticMeshComponent") "Ground")
                    (Variables|Default|SetBallState "NewEnumerator2")
                    (Rendering|Material|SetMaterial (Variables|Default|GetBall_Mesh) 0 "/Game/BallBP/Materials/Ball-Active.Ball-Active")
                    (goto _label Break)
                    (else
                      _)))))))
        (Variables|Default|SetBallState "NewEnumerator1")
        (Rendering|Material|SetMaterial (Variables|Default|GetBall_Mesh) 0 "/Game/BallBP/Materials/Ball-Inactive.Ball-Inactive")))))

(event Custom|EventStart_Client
  (Rendering|Material|SetMaterial (Variables|Default|GetBall_Mesh) 0 "/Game/BallBP/Materials/Ball-Stasis.Ball-Stasis")
  (Variables|Default|SetBallState "NewEnumerator3")
  (Physics|SetEnableGravity (Variables|Default|GetBall_Mesh) false)
  (Physics|SetSimulatePhysics (Variables|Default|GetBall_Mesh) false)
  (Class|PrimitiveComponent|SetUseCCD (Variables|Default|GetBall_Mesh) true "None"))

(event Custom|HitEvent_Client
  (Utilities|IsValid (stale Collision|EventHit Other)
    (:Is%20Valid
      (bind _asfirst_person_character (Utilities|Casting|CastToFirstPersonCharacter (stale Collision|EventHit Other)))
      (CallFunction|BallPickup _asfirst_person_character))))

(event EventBeginPlay
  (Networking|SwitchHasAuthority
    (:Authority
      (CallFunction|EventStartServer))
    (:Remote
      (CallFunction|EventStartClient))))

(event EventTick
  (params (DeltaSeconds :type Float%20%28single-precision%29))
  (Variables|Default|SetdeltaTime DeltaSeconds)
  (Networking|SwitchHasAuthority
    (:Authority
      (CallFunction|TickEventServer))))

(event Collision|EventHit
  (params (MyComp :type Primitive%20Component%20Object%20Reference) (Other :type Actor%20Object%20Reference) (OtherComp :type Primitive%20Component%20Object%20Reference) (bSelfMoved :type Boolean) (HitLocation :type Vector :default "0, 0, 0") (HitNormal :type Vector :default "0, 0, 0") (NormalImpulse :type Vector :default "0, 0, 0") (Hit :type Hit%20Result%20Structure%20%28by%20ref%29))
  (Networking|SwitchHasAuthority
    (:Authority
      (CallFunction|HitEventMulti))
    (:Remote
      (CallFunction|HitEventClient))))

(fn ConstructionScript)

(fn Explode
  (bind _ball_mesh (Variables|Default|GetBall_Mesh))
  (if (not (Variables|Default|GethasExploded))
    (Variables|Default|SethasExploded true)
    (Variables|Default|SetActiveOwner 0)
    (Physics|SetSimulatePhysics _ball_mesh false)
    (Physics|SetEnableGravity _ball_mesh false)
    (Transformation|AttachActorToActor 0 "None" "KeepRelative" "KeepRelative" "KeepRelative" true)
    (Transformation|AttachComponentToComponent (Variables|Default|GetBall_Mesh) 0 "None" "KeepRelative" "KeepRelative" "KeepRelative" true)
    (Variables|Default|SetBallState "NewEnumerator1")
    (bind _outactors (Collision|SphereOverlapActors (Transformation|GetWorldLocation (Variables|Default|GetBall_Mesh)) 1e+03 (Utilities|Array|MakeArray "ObjectTypeQuery4" "ObjectTypeQuery3" "ObjectTypeQuery1" "ObjectTypeQuery2" "ObjectTypeQuery6" "ObjectTypeQuery5" "ObjectTypeQuery7") 0))
    (for _array_element _outactors
      (bind _asfirst_person_character (Utilities|Casting|CastToFirstPersonCharacter _array_element))
      (Character|LaunchCharacter _asfirst_person_character (|GetExplosionVector _asfirst_person_character) true true))
    (Rendering|Material|SetMaterial (Variables|Default|GetBall_Mesh) 0 "/Game/BallBP/Materials/Ball-Exploded.Ball-Exploded")))

(fn BallPickup
  (params (Character :type First%20Person%20Character%20Object%20Reference))
  (bind _ball_mesh (Variables|Default|GetBall_Mesh))
  (bind _ball_mesh_2 (Variables|Default|GetBall_Mesh))
  (Utilities|IsValid (Variables|Default|GetActiveOwner)
    (:Is%20Valid
      (if (Utilities|IsIntercept Character)
        (Variables|Default|SetBallTimer 0.0)
        (else
          (Utilities|IsValid Character :!label _label
            (:Is%20Valid
              _)))))
    (:Is%20Not%20Valid
      (goto _label)))
  (Variables|Default|SetActiveOwner Character)
  (Development|PrintString (Utilities|GetDisplayName (Variables|Default|GetActiveOwner)) true true "(R=0.000000,G=0.660000,B=1.000000,A=1.000000)" 2e+01)
  (Development|PrintString (Utilities|GetDisplayName Character) true true "(R=0.040045,G=1.000000,B=0.000000,A=1.000000)" 2e+01)
  (Variables|/Game/FirstPersonBP/Blueprints/FirstPersonCharacter.FirstPersonCharacter_C|SetPassball (Variables|Default|GetActiveOwner) self)
  (Variables|Default|SetBallState "NewEnumerator0")
  (Rendering|Material|SetMaterial _ball_mesh 0 "/Game/BallBP/Materials/Ball-Active.Ball-Active")
  (Physics|SetEnableGravity _ball_mesh false)
  (Physics|SetSimulatePhysics _ball_mesh_2 false)
  (Collision|SetCollisionEnabled _ball_mesh_2 "QueryOnly")
  (CallFunction|BalltoHand))

(fn BalltoHand
  (bind _activeowner (Variables|Default|GetActiveOwner))
  (Development|PrintString (Utilities|GetDisplayName _activeowner) true true "(R=1.000000,G=0.064296,B=0.787177,A=1.000000)" 2e+01)
  (Transformation|AttachActorToActor _activeowner "None" "SnapToTarget" "KeepRelative" "KeepRelative" true)
  (Transformation|AttachComponentToComponent (Variables|Default|GetBall_Mesh) (Variables|/Game/FirstPersonBP/Blueprints/FirstPersonCharacter.FirstPersonCharacter_C|GetFirstPersonCamera _activeowner) "None" "SnapToTarget" "KeepRelative" "KeepRelative" true)
  (Transformation|SetRelativeTransform (Variables|Default|GetBall_Mesh) (Math|Transform|MakeTransform (Variables|Default|GetHandOffset)) false true))

(fn ThrowBall
  (params (ThrowForce :type Float%20%28single-precision%29) (ThrowDir :type Vector))
  (bind _ball_mesh (Variables|Default|GetBall_Mesh))
  (Collision|SetCollisionEnabled _ball_mesh "QueryAndPhysics")
  (Physics|SetEnableGravity _ball_mesh true)
  (Physics|SetSimulatePhysics _ball_mesh true)
  (Physics|AddImpulse _ball_mesh (* ThrowDir ThrowForce) "None" false)
  (Variables|Default|SetBallState "NewEnumerator1")
  (Rendering|Material|SetMaterial (Variables|Default|GetBall_Mesh) 0 "/Game/BallBP/Materials/Ball-Inactive.Ball-Inactive"))

(fn OnRepActiveOwner)