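; BP_Stun_Bullet is a stun gun actor that temporarily alters a Player's movement, despite its name containing no projectile logic in these graphs.
; On BeginPlay it multiplies the Player's MaxWalkSpeed and JumpZVelocity by speed and jump multipliers, then starts a one-shot StunTime timer.
; When the timer fires, it divides both values by the same multipliers rather than restoring cached originals, then destroys itself.
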(event Custom|Unstun%20Actor
  (bind _player (Variables|Default|GetPlayer))
  (bind _charactermovement (Variables|/Script/Engine.Character|GetCharacterMovement _player))
  (Variables|/Script/Engine.CharacterMovementComponent|SetMaxWalkSpeed _charactermovement (/ (Variables|/Script/Engine.CharacterMovementComponent|GetMaxWalkSpeed _charactermovement) (Variables|Default|GetSpeedMultiplier)))
  (Variables|/Script/Engine.CharacterMovementComponent|SetJumpZVelocity _charactermovement (/ (Variables|/Script/Engine.CharacterMovementComponent|GetJumpZVelocity _charactermovement) (Variables|Default|GetJumpMultiplier)))
  (Actor|DestroyActor))

(event Custom|Stun%20Actor
  (bind _player (Variables|Default|GetPlayer))
  (bind _charactermovement (Variables|/Script/Engine.Character|GetCharacterMovement _player))
  (Variables|/Script/Engine.CharacterMovementComponent|SetMaxWalkSpeed _charactermovement (* (Variables|/Script/Engine.CharacterMovementComponent|GetMaxWalkSpeed _charactermovement) (Variables|Default|GetSpeedMultiplier)))
  (Variables|/Script/Engine.CharacterMovementComponent|SetJumpZVelocity _charactermovement (* (Variables|/Script/Engine.CharacterMovementComponent|GetJumpZVelocity _charactermovement) (Variables|Default|GetJumpMultiplier))))

(event EventBeginPlay
  (CallFunction|StunActor)
  (Utilities|Time|SetTimerbyEvent (delegate Custom|Unstun%20Actor) (Variables|Default|GetStunTime)))

(fn ConstructionScript
  (|CallParentFunction))