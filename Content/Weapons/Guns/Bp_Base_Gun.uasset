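; Base gun Blueprint that responds to pickup use by firing or aiming, and destroys itself when its shots run out.
; Ranged guns line-trace from the owner's camera and spawn BulletClass only on a character hit, passing that character; non-ranged guns pass the owner.
; An AimLerp timeline blends the gun between grip socket and camera-relative offset, along with rotation and FOV.
; Ammo changes update the owner's HUD, with some updates limited to remote instances.
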(event Custom|Fire
  (bind (_start _end _type _ignore) (|Trace))
  ;[1 1 1] Actions
  (bind _result (Math|Integer|DecrementInt (Variables|Default|GetShots))
    (:%20%20
      (Default|UpdateAmmo (CallFunction|GetParent) _result)
      (if (Variables|Default|GetRanged?)
        (bind (_outhit _returnvalue) (Collision|LineTraceForObjects _start _end _type false _ignore "Persistent" true "(R=1.000000,G=0.000000,B=0.000000,A=1.000000)" "(R=0.000000,G=1.000000,B=0.000000,A=1.000000)" 1.0))
        (if _returnvalue
          (bind _asfirst_person_character (Utilities|Casting|CastToFirstPersonCharacter (.HitActor (Collision|BreakHitResult _outhit))))
          (CallFunction|MakeBullet _asfirst_person_character))
        (else
          (CallFunction|MakeBullet (CallFunction|GetParent))))
      (if (<= (Variables|Default|GetShots) 0)
        (Default|HideAmmo (CallFunction|GetParent) true)
        (CallFunction|DestroyonServer)))))

(event Custom|Make%20Bullet
  (params (Player :type First%20Person%20Character%20Object%20Reference))
  ;[1 1 1] Actions
  (Game|SpawnActorfromClass (Variables|Default|GetBullet%20Class) (Math|Transform|MakeTransform "0, 0, 0" (Transformation|GetWorldRotation (Variables|/Script/Passball_v2.Passball_v2Character|GetFirstPersonCameraComponent (CallFunction|GetParent))) "1,1,1") "Undefined" 0 Player 0))

(event Custom|Destroy%20On%20Server
  ;[1 1 1] Destroy
  (Class|BPIPickup|RemovePickup(Message) (CallFunction|GetParent))
  (CallFunction|DestroyonClient self))

(event Custom|Aim
  (params (Player :type Actor%20Object%20Reference) (Pressed? :type Boolean))
  ;[1 1 1] Actions
  (bind _asfirst_person_character (Utilities|Casting|CastToFirstPersonCharacter Player))
  (if Pressed?
    (bind _alpha (Timeline|Aim%20Lerp Play)
      (:Update
        (Transformation|SetActorLocation (.Aim%20Location (|AimOffsets _alpha _asfirst_person_character)) false true)
        (Transformation|SetActorRelativeRotation (.Aim%20Rotation (|AimOffsets _alpha _asfirst_person_character)))
        (Camera|SetFieldOfView (Variables|/Script/Passball_v2.Passball_v2Character|GetFirstPersonCameraComponent _asfirst_person_character) (.Aim%20FOV (|AimOffsets _alpha _asfirst_person_character)))))
    (else
      (Timeline|Aim%20Lerp Reverse))))

(event Custom|Destroy%20On%20Client
  (params (Actor :type Actor%20Object%20Reference))
  (bind _parentactor (CallFunction|GetParent))
  ;[1 1 1] Destroy
  (Camera|SetFieldOfView (Variables|/Script/Passball_v2.Passball_v2Character|GetFirstPersonCameraComponent _parentactor) (Variables|/Game/FirstPersonCPP/Blueprints/FirstPersonCharacter.FirstPersonCharacter_C|GetCamera%20FOV _parentactor))
  (Utilities|IsValid Actor
    (:Is%20Valid
      (Actor|DestroyActor Actor))))

(event Custom|HUD%20Update
  (bind _parentactor (CallFunction|GetParent))
  (Networking|SwitchHasAuthority
    (:Remote
      (Default|HideAmmo _parentactor false)
      (Default|UpdateAmmo _parentactor (Variables|Default|GetShots)))))

(event Custom|Update%20Ammo%20Multi
  (params (Shots :type Integer))
  (Networking|SwitchHasAuthority
    (:Remote
      ;[1 1 1] Actions
      (CallFunction|UpdateAmmoClient Shots))))

(event Custom|Update%20Ammo%20Client
  (params (NewParam :type Integer))
  (Default|UpdateAmmo (Variables|/Game/FirstPersonCPP/Blueprints/FirstPersonCharacter.FirstPersonCharacter_C|GetHUD%20Widget (CallFunction|GetParent)) NewParam))

(event EventUsePickup
  (params (Caller :type Actor%20Object%20Reference) (Main%20Pressed :type Boolean) (Main%20Released :type Boolean) (Alt%20Pressed :type Boolean) (Alt%20Released :type Boolean))
  (if Main%20Pressed
    (CallFunction|Fire)
    (elif (or Alt%20Pressed Alt%20Released)
      (CallFunction|Aim Caller Alt%20Pressed))))

(fn ConstructionScript
  (Components|Timeline|SetPlayRate (Variables|Default|GetAim%20Lerp) (Variables|Default|GetAim%20Blend%20Time)))

(fn GetParent
  (bind _bp_pickup (Variables|Default|GetBP_Pickup))
  (bind _childactor (Variables|/Script/Engine.ChildActorComponent|GetChildActor _bp_pickup))
  (bind (_asbp_pickup _bsuccess) (Utilities|Casting|CastToBP_Pickup _childactor))
  (return (select _bsuccess (Variables|/Game/Weapons/Components/BP_Pickup.BP_Pickup_C|GetParentActor _asbp_pickup) 0)))