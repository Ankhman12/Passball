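; BP_Pickup is a reusable pickup, used as a child actor, that lets a FirstPersonCharacter collect and use its parent actor.
; Sphere overlap or QueryPickup messages the character.
; Pickup relays through ServerPickup to ClientPickup, attaching the parent to the GripPoint socket and disabling sphere collision, and stops the bounce and spin timelines that move the parent.
; UsePickup forwards primary and alternate input to the parent actor.
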(event OnComponentBeginOverlap(PickupSphere)
  (params (OverlappedComponent :type Primitive%20Component%20Object%20Reference) (OtherActor :type Actor%20Object%20Reference) (OtherComp :type Primitive%20Component%20Object%20Reference) (OtherBodyIndex :type Integer) (bFromSweep :type Boolean) (SweepResult :type Hit%20Result%20Structure%20%28by%20ref%29))
  ;[1 1 1] Pickup Actions
  (bind _asfirst_person_character (Utilities|Casting|CastToFirstPersonCharacter OtherActor))
  (Class|BPIPickup|QueryPickup(Message) _asfirst_person_character self))

(event Custom|Server%20Pickup
  (params (Parent :type First%20Person%20Character%20Object%20Reference))
  ;[1 1 1] Pickup Actions
  (CallFunction|ClientPickup Parent))

(event Custom|Client%20Pickup
  (params (Parent :type First%20Person%20Character%20Object%20Reference))
  ;[1 1 1] Pickup Actions
  (Transformation|AttachComponentToComponent (Variables|/Script/Engine.Actor|GetRootComponent (Actor|GetParentActor)) (Variables|/Script/Engine.Character|GetMesh Parent) "GripPoint" "SnapToTarget" "SnapToTarget" "KeepWorld" true)
  (Collision|SetCollisionEnabled (Variables|Default|GetPickup%20Sphere) "NoCollision"))

(event EventBeginPlay
  (Variables|Default|SetOriginal%20Location (Transformation|GetActorLocation))
  (Variables|Default|SetOriginal%20Rotation (Transformation|GetActorRotation))
  (Components|Timeline|SetPlayRate (Variables|Default|GetBounce%20Animation) (Variables|Default|GetBounce%20Speed))
  (Components|Timeline|SetPlayRate (Variables|Default|GetRotate%20Animation) (Variables|Default|GetRotation%20Speed)))

(event EventPickup
  (params (Parent :type First%20Person%20Character%20Object%20Reference))
  ;[1 1 1] Pickup Actions
  (CallFunction|ServerPickup Parent)
  (Variables|Default|SetParentActor Parent)
  (Audio|Components|Audio|Stop (Variables|Default|GetBounce%20Animation)))

(event EventUsePickup
  (params (Caller :type Actor%20Object%20Reference) (Main%20Pressed :type Boolean) (Main%20Released :type Boolean) (Alt%20Pressed :type Boolean) (Alt%20Released :type Boolean))
  ;[1 1 1] Pickup Actions
  (Class|BPIPickup|UsePickup(Message) (Actor|GetParentActor) Caller Main%20Pressed Main%20Released Alt%20Pressed Alt%20Released))

(event EventQueryPickup
  (params (Caller :type Actor%20Object%20Reference))
  ;[1 1 1] Pickup Actions
  (Variables|Default|GetParentActor
    (:then)
    (:else
      (Class|BPIPickup|QueryPickup(Message) Caller self))))

(fn ConstructionScript)