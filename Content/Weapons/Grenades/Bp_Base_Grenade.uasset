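; Base grenade pickup that the player charges and throws, leaving Explode empty, presumably for child Blueprints.
; Holding either input builds throw force in a gated delay loop, though only main release closes it.
; Release detaches the mesh, enables physics and applies an impulse along the controller's forward vector.
; Timed grenades start their fuse on alt press (cooking) or main release; contact grenades explode once on hit after being thrown.
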(event OnComponentHit(Grenade)
  (params (HitComponent :type Primitive%20Component%20Object%20Reference) (OtherActor :type Actor%20Object%20Reference) (OtherComp :type Primitive%20Component%20Object%20Reference) (NormalImpulse :type Vector :default "0, 0, 0") (Hit :type Hit%20Result%20Structure%20%28by%20ref%29))
  ;[1 1 1] Grenade Use
  (if (and (Variables|Default|GetThrown) (Variables|Default|GetContactBased?))
    (Utilities|FlowControl|DoOnce false
      (:Completed
        (CallFunction|Explode)))))

(event Custom|Explode
  ;[1 1 1] Grenade Use
)

(event Custom|Server%20Launch
  ;[1 1 1] Grenade Use
  (|Launch))

(event Custom|Enable%20Physics
  (params (Parent :type First%20Person%20Character%20Object%20Reference))
  (bind _grenade (Variables|Default|GetGrenade))
  ;[1 1 1] Enable Physics
  (Transformation|DetachFromComponent (Variables|Default|GetGrenade) "KeepWorld" "KeepWorld" "KeepWorld" true)
  (Collision|SetCollisionEnabled _grenade "QueryAndPhysics")
  (Physics|SetSimulatePhysics _grenade true))

(event Custom|Destroy%20On%20Server
  ;[1 1 1] Destroy Actor
  (CallFunction|DestroyonClient self))

(event Custom|Destroy%20On%20Client
  (params (Actor :type Actor%20Object%20Reference))
  ;[1 1 1] Destroy Actor
  (Utilities|IsValid Actor
    (:Is%20Valid
      (Actor|DestroyActor Actor))))

(event Custom|Server%20Use
  ;[1 1 1] Grenade Use
  (if (Variables|Default|GetTimed?)
    (Utilities|Time|SetTimerbyEvent (delegate Custom|Explode) (Variables|Default|GetTime))))

(event EventUsePickup
  (params (Caller :type Actor%20Object%20Reference) (Main%20Pressed :type Boolean) (Main%20Released :type Boolean) (Alt%20Pressed :type Boolean) (Alt%20Released :type Boolean))
  ;[1 1 1] Grenade Throw
  (if (or Main%20Pressed Alt%20Pressed)
    (|IncreaseThrow :!label _label)
    (if Alt%20Pressed
      (CallFunction|ServerUse))
    (elif Main%20Released
      (Utilities|FlowControl|Sequence
        (:then_0
          (goto _label Close))
        (:then_1
          (CallFunction|ServerLaunch)
          (CallFunction|ServerUse)
          (Class|BPIPickup|RemovePickup(Message) Caller)
          (Variables|Default|SetThrown true)))
      (elif Alt%20Released
        (CallFunction|ServerLaunch)
        (Class|BPIPickup|RemovePickup(Message) Caller)
        (Variables|Default|SetThrown true)))))

(fn ConstructionScript)