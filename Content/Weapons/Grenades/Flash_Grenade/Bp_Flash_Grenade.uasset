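; Flash grenade that blinds first-person characters near its explosion, extending a parent grenade's explode logic.
; Explode sphere-traces for pawns and passes them to Flash, which requires a camera angle within limits and an unblocked line trace.
; Each qualifying character is flashed at an angle-derived intensity, as is any character still holding the grenade.
; It then destroys itself via a client call, or a server call when the trace finds nothing.
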(event Custom|Flash
  (params (Actors :type Array%20of%20First%20Person%20Character%20Object%20References))
  (bind _returnvalue (Actor|GetAttachParentActor))
  ;[1 1 1] Flash Effect
  (for _array_element Actors
    ;;[1 1 1] Check Line Of Sight
    (if (and (<= (CallFunction|AngleBetween2Vectors (Math|Vector|GetForwardVector (Variables|/Script/Passball_v2.Passball_v2Character|GetFirstPersonCameraComponent _array_element)) (Math|Vector|GetUnitDirection(Vector) (Transformation|GetActorLocation _array_element) (Transformation|GetActorLocation))) (Variables|Default|GetMax%20Angle)) (>= (CallFunction|AngleBetween2Vectors (Math|Vector|GetForwardVector (Variables|/Script/Passball_v2.Passball_v2Character|GetFirstPersonCameraComponent _array_element)) (Math|Vector|GetUnitDirection(Vector) (Transformation|GetActorLocation _array_element) (Transformation|GetActorLocation))) (Variables|Default|GetMin%20Angle)))
      (bind _outhit (Collision|LineTraceByChannel (Transformation|GetActorLocation) (Transformation|GetActorLocation _array_element) "TraceTypeQuery2" false (Utilities|Array|MakeArray (Actor|GetAttachParentActor)) "Persistent"))
      (if (== (.HitActor (Collision|BreakHitResult _outhit)) _array_element)
        (Default|Flash _array_element (CallFunction|IntensityBasedonAngle (CallFunction|AngleBetween2Vectors (Math|Vector|GetForwardVector (Variables|/Script/Passball_v2.Passball_v2Character|GetFirstPersonCameraComponent _array_element)) (Math|Vector|GetUnitDirection(Vector) (Transformation|GetActorLocation _array_element) (Transformation|GetActorLocation))))))))
  ;;[1 1 1] Flash Player if Held
  (Utilities|IsValid _returnvalue
    (:Is%20Valid
      (Default|Flash (.AsFirst%20Person%20Character (Utilities|Casting|CastToFirstPersonCharacter _returnvalue)) (CallFunction|IntensityBasedonAngle 0.0)))))

(event EventExplode
  (bind _returnvalue (Transformation|GetActorLocation))
  ;[1 1 1] Grenade Effects
  (|CallParentFunction)
  (bind (_outhits _returnvalue_2) (Collision|MultiSphereTraceForObjects _returnvalue _returnvalue (Variables|Default|GetRadius) (Utilities|Array|MakeArray "ObjectTypeQuery3") false 0 "None"))
  (if _returnvalue_2
    (for _array_element _outhits
      (bind _asfirst_person_character (Utilities|Casting|CastToFirstPersonCharacter (.HitActor (Collision|BreakHitResult _array_element))))
      (Utilities|Array|Add (Variables|Default|GetHit%20Players) _asfirst_person_character))
    (CallFunction|Flash (Variables|Default|GetHit%20Players))
    (Utilities|FlowControl|Delay 0.1)
    (CallFunction|DestroyonClient self)
    (else
      (CallFunction|DestroyonServer))))

(fn ConstructionScript
  (|CallParentFunction))

(fn AngleBetween2Vectors
  (params (Vector%201 :type Vector) (Vector%202 :type Vector))
  (return (Class|KismetMathLibrary|DegAcos (/ (Math|Vector|DotProduct Vector%201 Vector%202) (* (Math|Vector|VectorLength Vector%201) (Math|Vector|VectorLength Vector%202))))))

(fn IntensityBasedonAngle
  (params (Angle :type Float%20%28single-precision%29))
  (bind _min_angle (Variables|Default|GetMin%20Angle))
  (bind _intensity_difference (Variables|Default|GetIntensity%20Difference))
  (bind _returnvalue (Math|Float|MakeLiteralFloat _intensity_difference))
  (return (+ (* (Variables|Default|GetFlash%20Intensity) (Math|Float|SelectFloat (- 1.0 (Math|Float|NormalizetoRange Angle _min_angle (+ _min_angle _returnvalue))) (Math|Float|NormalizetoRange Angle 0.0 (+ (Variables|Default|GetMax%20Angle) _returnvalue)) (< Angle 0.0))) 1.0)))