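; Stun grenade burst that slows first-person characters caught in its blast radius for a set time.
; On explosion it runs the parent logic, sphere-traces for pawns with debug drawing, stores the hits, and hides the grenade mesh.
; Stun multiplies each character's walk, sprint, run and wall-run speeds and sprint acceleration by SpeedMultiplier.
; A timer later divides the same values back for the stored hits, then destroys the actor through DestroyOnClient.
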(event Custom|Stun
  ;[1 1 1] Stun Effects
  (Variables|Default|SetStunning true)
  (for _array_element (Variables|Default|GetHit%20Pawns)
    (bind _asfirst_person_character (Utilities|Casting|CastToFirstPersonCharacter (.HitActor (Collision|BreakHitResult _array_element))))
    (CallFunction|StunActor (.AsMy%20Character%20Movement%20Component (Utilities|Casting|CastToMyCharacterMovementComponent (Variables|/Script/Engine.Character|GetCharacterMovement _asfirst_person_character))))))

(event Custom|Stun%20Actor
  (params (Movement%20Component :type My%20Character%20Movement%20Component%20Object%20Reference))
  ;[1 1 1] Stun Effects
  (Variables|/Script/Engine.CharacterMovementComponent|SetMaxWalkSpeed Movement%20Component (* (Variables|/Script/Engine.CharacterMovementComponent|GetMaxWalkSpeed Movement%20Component) (Variables|Default|GetSpeedMultiplier)))
  (Variables|/Script/Passball_v2.MyCharacterMovementComponent|SetSprintSpeed Movement%20Component (* (Variables|/Script/Passball_v2.MyCharacterMovementComponent|GetSprintSpeed Movement%20Component) (Variables|Default|GetSpeedMultiplier)))
  (Variables|/Script/Passball_v2.MyCharacterMovementComponent|SetRunSpeed Movement%20Component (* (Variables|/Script/Passball_v2.MyCharacterMovementComponent|GetRunSpeed Movement%20Component) (Variables|Default|GetSpeedMultiplier)))
  (Variables|/Script/Passball_v2.MyCharacterMovementComponent|SetWallRunSpeed Movement%20Component (* (Variables|/Script/Passball_v2.MyCharacterMovementComponent|GetWallRunSpeed Movement%20Component) (Variables|Default|GetSpeedMultiplier)))
  (Variables|/Script/Passball_v2.MyCharacterMovementComponent|SetSprintAcceleration Movement%20Component (* (Variables|/Script/Passball_v2.MyCharacterMovementComponent|GetSprintAcceleration Movement%20Component) (Variables|Default|GetSpeedMultiplier)))
  (Development|SetHiddeninGame (Variables|Default|GetGrenade) true false))

(event Custom|Unstun%20Actor
  (params (Movement%20Component :type My%20Character%20Movement%20Component%20Object%20Reference))
  ;[1 1 1] Stop Stun
  (Variables|/Script/Engine.CharacterMovementComponent|SetMaxWalkSpeed Movement%20Component (/ (Variables|/Script/Engine.CharacterMovementComponent|GetMaxWalkSpeed Movement%20Component) (Variables|Default|GetSpeedMultiplier)))
  (Variables|/Script/Passball_v2.MyCharacterMovementComponent|SetSprintSpeed Movement%20Component (/ (Variables|/Script/Passball_v2.MyCharacterMovementComponent|GetSprintSpeed Movement%20Component) (Variables|Default|GetSpeedMultiplier)))
  (Variables|/Script/Passball_v2.MyCharacterMovementComponent|SetRunSpeed Movement%20Component (/ (Variables|/Script/Passball_v2.MyCharacterMovementComponent|GetRunSpeed Movement%20Component) (Variables|Default|GetSpeedMultiplier)))
  (Variables|/Script/Passball_v2.MyCharacterMovementComponent|SetWallRunSpeed Movement%20Component (/ (Variables|/Script/Passball_v2.MyCharacterMovementComponent|GetWallRunSpeed Movement%20Component) (Variables|Default|GetSpeedMultiplier)))
  (Variables|/Script/Passball_v2.MyCharacterMovementComponent|SetSprintAcceleration Movement%20Component (/ (Variables|/Script/Passball_v2.MyCharacterMovementComponent|GetSprintAcceleration Movement%20Component) (Variables|Default|GetSpeedMultiplier))))

(event Custom|Stop%20Stun
  ;[1 1 1] Stop Stun
  (Variables|Default|SetStunning false)
  (for _array_element (Variables|Default|GetHit%20Pawns)
    (bind _asfirst_person_character (Utilities|Casting|CastToFirstPersonCharacter (.HitActor (Collision|BreakHitResult _array_element))))
    (CallFunction|UnstunActor (.AsMy%20Character%20Movement%20Component (Utilities|Casting|CastToMyCharacterMovementComponent (Variables|/Script/Engine.Character|GetCharacterMovement _asfirst_person_character)))))
  (Utilities|FlowControl|Delay 0.2)
  (CallFunction|DestroyonClient self))

(event EventExplode
  (bind _returnvalue (Transformation|GetActorLocation))
  ;[1 1 1] Grenade Explosion
  (|CallParentFunction)
  (bind (_outhits _returnvalue_2) (Collision|MultiSphereTraceForObjects _returnvalue _returnvalue (Variables|Default|GetRadius) (Utilities|Array|MakeArray "ObjectTypeQuery3") false 0 "ForDuration"))
  (if _returnvalue_2
    (Variables|Default|SetHit%20Pawns _outhits))
  (CallFunction|Stun)
  (Development|SetHiddeninGame (Variables|Default|GetGrenade) true false)
  (Utilities|Time|SetTimerbyEvent (delegate Custom|Stop%20Stun) (Variables|Default|GetStunTime)))

(fn ConstructionScript
  (|CallParentFunction))