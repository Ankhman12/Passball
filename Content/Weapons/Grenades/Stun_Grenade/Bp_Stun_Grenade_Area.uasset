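; Stun grenade that, on explosion, creates a timed area that slows first-person characters inside it.
; A sphere trace catches initial pawns, while overlap events track characters entering or leaving during the stun.
; Stunning multiplies movement component speeds and sprint acceleration by SpeedMultiplier, and unstunning divides them back.
; Timelines scale the visible and post-process spheres on show and hide, but the final destroy call is never reached.
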(event OnComponentBeginOverlap(StunCollision)
  (params (OverlappedComponent :type Primitive%20Component%20Object%20Reference) (OtherActor :type Actor%20Object%20Reference) (OtherComp :type Primitive%20Component%20Object%20Reference) (OtherBodyIndex :type Integer) (bFromSweep :type Boolean) (SweepResult :type Hit%20Result%20Structure%20%28by%20ref%29))
  ;[1 1 1] Stun Effects
  (if (Variables|Default|GetStunning)
    (bind _asfirst_person_character (Utilities|Casting|CastToFirstPersonCharacter OtherActor))
    (CallFunction|StunActor (.AsMy%20Character%20Movement%20Component (Utilities|Casting|CastToMyCharacterMovementComponent (Variables|/Script/Engine.Character|GetCharacterMovement _asfirst_person_character))))
    (Utilities|Array|AddUnique (Variables|Default|GetStunnedActors) OtherActor)))

(event OnComponentEndOverlap(StunCollision)
  (params (OverlappedComponent :type Primitive%20Component%20Object%20Reference) (OtherActor :type Actor%20Object%20Reference) (OtherComp :type Primitive%20Component%20Object%20Reference) (OtherBodyIndex :type Integer))
  ;[1 1 1] Stun Effects
  (if (Variables|Default|GetStunning)
    (bind _asfirst_person_character (Utilities|Casting|CastToFirstPersonCharacter OtherActor))
    (CallFunction|UnstunActor (.AsMy%20Character%20Movement%20Component (Utilities|Casting|CastToMyCharacterMovementComponent (Variables|/Script/Engine.Character|GetCharacterMovement _asfirst_person_character))))
    (Utilities|Array|RemoveItem (Variables|Default|GetStunnedActors) OtherActor)))

(event Custom|Stun
  ;[1 1 1] Stun Effects
  (CallFunction|ShowSphere)
  (Variables|Default|SetStunning true)
  (CallFunction|StunFirstActors (Variables|Default|GetStunnedActors)))

(event Custom|Stop%20Stun
  ;[1 1 1] Stop Stun
  (Variables|Default|SetStunning false)
  (for _array_element (Variables|Default|GetStunnedActors)
    (bind _asfirst_person_character (Utilities|Casting|CastToFirstPersonCharacter _array_element))
    (CallFunction|UnstunActor (.AsMy%20Character%20Movement%20Component (Utilities|Casting|CastToMyCharacterMovementComponent (Variables|/Script/Engine.Character|GetCharacterMovement _asfirst_person_character)))))
  (CallFunction|HideSphere)
  (Utilities|FlowControl|Delay 0.2 :!label _label)
  (if (Audio|Components|Audio|IsPlaying (Variables|Default|GetStun%20Sphere%20Compression))
    (goto _label)))

(event Custom|Hide%20Sphere
  (bind _radius (Variables|Default|GetRadius))
  ;[1 1 1] Stop Stun
  (bind _alpha (Timeline|Stun%20Sphere%20Compression PlayFromStart)
    (:Update
      (Transformation|SetWorldScale3D (Variables|Default|GetStun%20Sphere) (Math|Vector|Lerp(Vector) "1.000000,1.000000,1.000000" (Math|Vector|MakeVector _radius _radius _radius) _alpha)))))

(event Custom|Stun%20First%20Actors
  (params (Actors :type Array%20of%20Actor%20Object%20References))
  ;[1 1 1] Stun Effects
  (for _array_element Actors
    (bind _asfirst_person_character (Utilities|Casting|CastToFirstPersonCharacter _array_element))
    (CallFunction|StunActor (.AsMy%20Character%20Movement%20Component (Utilities|Casting|CastToMyCharacterMovementComponent (Variables|/Script/Engine.Character|GetCharacterMovement _asfirst_person_character))))))

(event Custom|Stun%20Actor
  (params (Movement%20Component :type My%20Character%20Movement%20Component%20Object%20Reference))
  ;[1 1 1] Stun Effects
  (Variables|/Script/Engine.CharacterMovementComponent|SetMaxWalkSpeed Movement%20Component (* (Variables|/Script/Engine.CharacterMovementComponent|GetMaxWalkSpeed Movement%20Component) (Variables|Default|GetSpeedMultiplier)))
  (Variables|/Script/Passball_v2.MyCharacterMovementComponent|SetSprintSpeed Movement%20Component (* (Variables|/Script/Passball_v2.MyCharacterMovementComponent|GetSprintSpeed Movement%20Component) (Variables|Default|GetSpeedMultiplier)))
  (Variables|/Script/Passball_v2.MyCharacterMovementComponent|SetRunSpeed Movement%20Component (* (Variables|/Script/Passball_v2.MyCharacterMovementComponent|GetRunSpeed Movement%20Component) (Variables|Default|GetSpeedMultiplier)))
  (Variables|/Script/Passball_v2.MyCharacterMovementComponent|SetWallRunSpeed Movement%20Component (* (Variables|/Script/Passball_v2.MyCharacterMovementComponent|GetWallRunSpeed Movement%20Component) (Variables|Default|GetSpeedMultiplier)))
  (Variables|/Script/Passball_v2.MyCharacterMovementComponent|SetSprintAcceleration Movement%20Component (* (Variables|/Script/Passball_v2.MyCharacterMovementComponent|GetSprintAcceleration Movement%20Component) (Variables|Default|GetSpeedMultiplier)))
  (Development|SetHiddeninGame (Variables|Default|GetGrenade) true false))

(event Custom|Unstun%20Actor
  (params (Movement%20Component :type My%20Character%20Movement%20Component%20Object%20Reference))
  ;[1 1 1] Stop Stun
  (Variables|/Script/Engine.CharacterMovementComponent|SetMaxWalkSpeed Movement%20Component (/ (Variables|/Script/Engine.CharacterMovementComponent|GetMaxWalkSpeed Movement%20Component) (Variables|Default|GetSpeedMultiplier)))
  (Variables|/Script/Passball_v2.MyCharacterMovementComponent|SetSprintSpeed Movement%20Component (/ (Variables|/Script/Passball_v2.MyCharacterMovementComponent|GetSprintSpeed Movement%20Component) (Variables|Default|GetSpeedMultiplier)))
  (Variables|/Script/Passball_v2.MyCharacterMovementComponent|SetRunSpeed Movement%20Component (/ (Variables|/Script/Passball_v2.MyCharacterMovementComponent|GetRunSpeed Movement%20Component) (Variables|Default|GetSpeedMultiplier)))
  (Variables|/Script/Passball_v2.MyCharacterMovementComponent|SetWallRunSpeed Movement%20Component (/ (Variables|/Script/Passball_v2.MyCharacterMovementComponent|GetWallRunSpeed Movement%20Component) (Variables|Default|GetSpeedMultiplier)))
  (Variables|/Script/Passball_v2.MyCharacterMovementComponent|SetSprintAcceleration Movement%20Component (/ (Variables|/Script/Passball_v2.MyCharacterMovementComponent|GetSprintAcceleration Movement%20Component) (Variables|Default|GetSpeedMultiplier))))

(event Custom|Show%20Sphere
  (bind _radius (Variables|Default|GetRadius))
  ;[1 1 1] Stun Effects
  (Physics|SetSimulatePhysics (Variables|Default|GetGrenade) false)
  (Development|SetHiddeninGame (Variables|Default|GetStun%20Sphere) false false)
  (Variables|/Script/Engine.PostProcessComponent|SetbEnabled (Variables|Default|GetPostProcess) true)
  (bind _alpha (Timeline|Timeline_0 PlayFromStart)
    (:Update
      (Transformation|SetWorldScale3D (Variables|Default|GetPP_Sphere) (Math|Vector|Lerp(Vector) "1.000000,1.000000,1.000000" (Math|Vector|MakeVector _radius _radius _radius) _alpha)))))

(event EventExplode
  (bind _returnvalue (Transformation|GetActorLocation))
  (|CallParentFunction)
  (bind (_outhits _returnvalue_2) (Collision|MultiSphereTraceForObjects _returnvalue _returnvalue (Variables|Default|GetRadius) (Utilities|Array|MakeArray "ObjectTypeQuery3") false 0 "None"))
  (if _returnvalue_2
    (for _array_element _outhits
      (Utilities|Array|AddUnique (Variables|Default|GetStunnedActors) (.HitActor (Collision|BreakHitResult _array_element)))))
  (CallFunction|Stun)
  (Utilities|Time|SetTimerbyEvent (delegate Custom|Stop%20Stun) (Variables|Default|GetStunTime)))

(fn ConstructionScript
  (|CallParentFunction))